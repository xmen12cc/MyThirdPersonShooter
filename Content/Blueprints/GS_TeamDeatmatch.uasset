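; Team deathmatch state Blueprint that tracks living members of Team A and Team B and declares the winner.
; DecreaseTeamNumber decrements the chosen team's count; at zero it shows a winner widget for the opposing team, then pauses the game after a short delay.
; Otherwise UpdateWidget writes both counts to the HUD of player 0's BP_ThirdPersonCharacter, as it also does shortly after BeginPlay.
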(event Custom|DecreaseTeamNumber
  (params (Tean%20A :type Boolean))
  (if Tean%20A
    (bind _result (Math|Integer|DecrementInt (Variables|Default|GetnumberOfTeamAalive))
      (:%20%20
        (if (<= _result 0)
          (bind _returnvalue (UserInterface|CreateWidget "/Game/TeamWinner_Widget.TeamWinner_Widget_C"))
          (Variables|/Script/UMG.TextBlock|SetText (Variables|/Game/TeamWinner_Widget.TeamWinner_Widget_C|GetTeamWinnerText _returnvalue) "Team B has won")
          (UserInterface|Viewport|AddtoViewport _returnvalue 0)
          (Utilities|FlowControl|Delay 2.0 :!label _label)
          (Game|SetGamePaused true)
          (else
            (CallFunction|UpdateWidget :!label _label_2)))))
    (else
      (bind _result_2 (Math|Integer|DecrementInt (Variables|Default|GetnumberOfTeamBalive))
        (:%20%20
          (if (<= _result_2 0)
            (bind _returnvalue_2 (UserInterface|CreateWidget "/Game/TeamWinner_Widget.TeamWinner_Widget_C"))
            (Variables|/Script/UMG.TextBlock|SetText (Variables|/Game/TeamWinner_Widget.TeamWinner_Widget_C|GetTeamWinnerText _returnvalue_2) "Team A has won")
            (UserInterface|Viewport|AddtoViewport _returnvalue_2 0)
            (goto _label)
            (else
              (goto _label_2))))))))

(event Custom|UpdateWidget
  ;[1 1 1] UpdateWidget
  (bind _asbp_third_person_character (Utilities|Casting|CastToBP_ThirdPersonCharacter (Game|GetPlayerCharacter 0)))
  (Variables|/Script/UMG.TextBlock|SetText (Variables|/Game/WB_HUD.WB_HUD_C|GetTeamA (Variables|/Game/ThirdPerson/Blueprints/BP_ThirdPersonCharacter.BP_ThirdPersonCharacter_C|GetHUD _asbp_third_person_character)) (Utilities|Text|FormatText "TEAM A: {value}" (Variables|Default|GetnumberOfTeamAalive)))
  (Variables|/Script/UMG.TextBlock|SetText (Variables|/Game/WB_HUD.WB_HUD_C|GetTeamB (Variables|/Game/ThirdPerson/Blueprints/BP_ThirdPersonCharacter.BP_ThirdPersonCharacter_C|GetHUD _asbp_third_person_character)) (Utilities|Text|FormatText "TEAM B: {value}" (Variables|Default|GetnumberOfTeamBalive))))

(event EventBeginPlay
  (Utilities|FlowControl|Delay 0.2)
  (CallFunction|UpdateWidget))

(fn ConstructionScript)