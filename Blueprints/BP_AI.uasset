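; AI soldier for team deathmatch that patrols, hunts enemies and fights with a rifle.
; It roams random reachable points until PawnSensing spots another team's pawn via BPI_TeamInteraction, then chases with AIMoveTo and shoots.
; A montage notify fires a damaging line trace from the muzzle, and a miss resumes patrol.
; Lethal damage ragdolls it and updates the game state's team count, while Tick updates the health bar and turns widgets toward the camera.
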(event OnSeePawn(PawnSensing)
  (params (Pawn :type Pawn%20Object%20Reference))
  ;[1 1 1] OnSeePawn (PawnSensing
  (if (Utilities|DoesObjectImplementInterface Pawn "/Game/Blueprints/BPI_TeamInteraction.BPI_TeamInteraction_C")
    (bind _team (Class|BPITeamInteraction|GetTeam(Message) Pawn))
    (if (!= _team (Math|Conversions|ToInteger(Byte) (Variables|Default|Getteam)))
      (bind _asbp_ai (Utilities|Casting|CastToBP_AI Pawn)
        (:then
          (if (Variables|BP_AI_C|GetisDead? _asbp_ai)
            (CallFunction|SearchAround)
            (else
              (CallFunction|ChaseTarget Pawn :!label _label)
              (Variables|Default|SethasSeenTarget? true))))
        (:CastFailed
          (goto _label))))))

(event Custom|Search%20Around
  ;[0.05098 0.05098 0.05098] SearchAround
  (if (not (Variables|Default|GethasSeenTarget?))
    (AI|AIMoveTo self (.RandomLocation (AI|Navigation|GetRandomReachablePointinRadius (Transformation|GetActorLocation) 2e+03 0 0)) 0 7.5e+02 false
      (:OnSuccess
        (Utilities|FlowControl|Delay 1.0)
        (CallFunction|SearchAround)))))

(event Custom|JogAround
  ;[1 1 1] Jog around and patrol
  (CallFunction|SearchAround)
  (Utilities|FlowControl|Sequence
    (:then_0
      ;[1 1 1] SetTeamText
      (if (== (Variables|Default|Getteam) 1)
        (Components|SkeletalMesh|SetSkeletalMeshAsset (Variables|Character|GetMesh) "/Game/SCK_Casual01/Models/Premade_Characters/MESH_PC_01B.MESH_PC_01B")
        (bind _asteam_indicator_widget (Utilities|Casting|CastToTeamIndicatorWidget (UserInterface|GetWidget (Variables|Default|GetTeamIndicator))))
        (Variables|/Script/UMG.TextBlock|SetText (Variables|/Game/TeamIndicatorWidget.TeamIndicatorWidget_C|GetTeamText _asteam_indicator_widget) "TEAM B")))
    (:then_1
      (Utilities|FlowControl|Delay 0.25 :!label _label)
      (if (Variables|Default|GethasSeenTarget?)
        (CallFunction|SearchAround)
        (Variables|Default|SethasSeenTarget? false)
        (goto _label)))))

(event Custom|ChaseTarget
  (params (TargetActor :type Actor%20Object%20Reference))
  ;[1 1 1] ChaseTarget
  (AI|AIMoveTo self "0, 0, 0" TargetActor 7.5e+02 false
    (:OnSuccess
      (CallFunction|Shoot TargetActor))))

(event Custom|Shoot
  (params (TargetActor :type Actor%20Object%20Reference))
  (bind _weapon (Variables|Default|GetWeapon))
  (bind _mesh (Variables|Character|GetMesh))
  (bind _returnvalue (Transformation|GetSocketTransform _weapon "b_gun_muzzleflash" "RTS_World"))
  (bind _returnvalue_2 (Transformation|GetWorldRotation _mesh))
  ;[1 1 1] Shoot
  (if (not (Variables|Default|GetisDead?))
    (Pawn|SetControlRotation (Pawn|GetController) (Math|Rotator|FindLookatRotation (Transformation|GetActorLocation) (Transformation|GetActorLocation TargetActor)))
    (Animation|Montage|PlayMontage (Variables|Character|GetMesh) "/Game/ShooterAnimations/Fire_Rifle_Ironsights_Montage.Fire_Rifle_Ironsights_Montage"
      (:OnNotifyBegin
        (Effects|SpawnEmitterAttached "/Game/InfinityBladeEffects/Effects/FX_Monsters/FX_Monster_Gruntling/Master/P_BackPack_MuzzleFlash.P_BackPack_MuzzleFlash" (Variables|Default|GetWeapon) "b_gun_muzzleflash" (.location _returnvalue) _returnvalue_2 "0.100000,0.100000,0.100000" "KeepWorldPosition")
        (Audio|PlaySoundatLocation "/Game/Sounds/MS_RifleFire.MS_RifleFire" (Transformation|GetActorLocation) "0, 0, 0" 0.65 1.0 0.0 0 0 0 0)
        (bind (_outhit _returnvalue_3) (Collision|LineTraceByChannel (.location _returnvalue) (+ (.location _returnvalue) (* (Math|Vector|GetRightVector _returnvalue_2) 3e+03)) "TraceTypeQuery1" false 0 "None"))
        (if _returnvalue_3
          (Game|Damage|ApplyDamage (.HitActor (Collision|BreakHitResult _outhit)) 1e+01 0 0)
          (Effects|SpawnEmitteratLocation "/Game/InfinityBladeEffects/Effects/FX_Monsters/FX_Monster_Troll/death/P_TrollDeathImpact.P_TrollDeathImpact" (.ImpactPoint (Collision|BreakHitResult _outhit)) (Math|Rotator|MakeRotfromX (.Normal (Collision|BreakHitResult _outhit))) "0.650000,0.650000,0.650000")
          (Audio|PlaySoundatLocation "/Game/Sounds/MS_hitConcrete.MS_hitConcrete" (Transformation|GetActorLocation) "0, 0, 0" 0.35 1.0 0.0 0 0 0 0)
          (else
            (Variables|Default|SethasSeenTarget? false)
            (CallFunction|JogAround)))))))

(event Game|Damage|EventAnyDamage
  (params (Damage :type Float%20%28single-precision%29) (DamageType :type Damage%20Type%20Object%20Reference) (InstigatedBy :type Controller%20Object%20Reference) (DamageCauser :type Actor%20Object%20Reference))
  ;[0.05098 0.05098 0.05098] Health
  (Variables|Default|Sethealth (- (Variables|Default|Gethealth) Damage))
  (if (<= (Variables|Default|Gethealth) 0.0)
    (Utilities|FlowControl|DoOnce false
      (:Completed
        (Physics|SetSimulatePhysics (Variables|Character|GetMesh) true)
        (Pawn|Components|CharacterMovement|SetMovementMode (Variables|Character|GetCharacterMovement) "MOVE_None" 0)
        (Variables|Default|SetisDead? true)
        (Rendering|SetVisibility (Variables|Default|GetHealthBar_Widget) false false)
        (bind _asgs_team_deatmatch (Utilities|Casting|CastToGS_TeamDeatmatch (Game|GetGameState)))
        (Default|DecreaseTeamNumber _asgs_team_deatmatch (== (Variables|Default|Getteam) 0))))))

(event EventTick
  (params (DeltaSeconds :type Float%20%28single-precision%29))
  ;[1 1 1] OnTick and widgets
  (bind _asai_health_bar (Utilities|Casting|CastToAI_HealthBar (UserInterface|GetWidget (Variables|Default|GetHealthBar_Widget))))
  (Progress|SetPercent (Variables|/Game/AI_HealthBar.AI_HealthBar_C|GetHealthBar _asai_health_bar) (/ (Variables|Default|Gethealth) 1e+02))
  (Transformation|SetWorldRotation (Variables|Default|GetHealthBar_Widget) (Math|Rotator|FindLookatRotation (Transformation|GetActorLocation) (Camera|GetCameraLocation (Game|GetPlayerCameraManager 0))) false false))

(event EventSetTeam
  (params (Team :type E_Teams%20Enum :default "NewEnumerator0"))
  ;[1 1 1] SetTeam
  (Variables|Default|Setteam Team))

(event EventBeginPlay
  ;[1 1 1] BeginPlay And Jog around
  (CallFunction|JogAround))

(fn ConstructionScript)

(fn GetTeam
  (return (Variables|Default|Getteam)))